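; Player parkour character with double jump, wall running, ledge climbing and ladder climbing.
; A DoN gate reset on landing limits jump launches, while overlapping "RunWall" actors starts a timeline that, with Space held, zeroes gravity and pushes along the camera direction.
; A per-tick trace finds "Climb_Wall_Able" surfaces, launching upward early in a Space hold and blocking move and look input.
; Near ladders, the Climbing action toggles flying movement along the up vector.
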(event OnComponentBeginOverlap(wallRunningCollision)
  (params (OverlappedComponent :type Primitive%20Component%20Object%20Reference) (OtherActor :type Actor%20Object%20Reference) (OtherComp :type Primitive%20Component%20Object%20Reference) (OtherBodyIndex :type Integer) (bFromSweep :type Boolean) (SweepResult :type Hit%20Result%20Structure%20%28by%20ref%29))
  (bind _charactermovement (Variables|Character|GetCharacterMovement))
  (bind _charactermovement_2 (Variables|Character|GetCharacterMovement))
  ;[1 1 1] Wall Running
  (Variables|Default|SetPlayerDirection (Math|Vector|GetForwardVector (Variables|Default|GetCamera)))
  (if (Actor|ActorHasTag OtherActor "RunWall")
    (Variables|Default|SetOnWall? true)
    (Timeline|WR_Timeline Play
      (:Update
        (if (> (Class|PlayerController|GetInputKeyTimeDown (Game|GetPlayerController 0) "SpaceBar") 0.0)
          (if (Variables|Default|GetOnWall?)
            (Variables|/Script/Engine.CharacterMovementComponent|SetGravityScale _charactermovement_2 0.0)
            (Class|MovementComponent|SetPlaneConstraintNormal _charactermovement_2 "0, 0,1.000000")
            (Physics|AddForce _charactermovement_2 (* (Variables|Default|GetPlayerDirection) 4000))
            (else
              (Variables|/Script/Engine.CharacterMovementComponent|SetGravityScale _charactermovement 1.0)
              (Class|MovementComponent|SetPlaneConstraintNormal _charactermovement "0, 0,0.000000")
              (Variables|Default|SetOnWall? false))))))))

(event OnComponentEndOverlap(wallRunningCollision)
  (params (OverlappedComponent :type Primitive%20Component%20Object%20Reference) (OtherActor :type Actor%20Object%20Reference) (OtherComp :type Primitive%20Component%20Object%20Reference) (OtherBodyIndex :type Integer))
  (bind _charactermovement (Variables|Character|GetCharacterMovement))
  (bind _charactermovement_2 (Variables|Character|GetCharacterMovement))
  ;[1 1 1] Wall Running
  (Utilities|FlowControl|Sequence
    (:then_0
      (Timeline|WR_Timeline Stop
        (:Update
          (if (> (Class|PlayerController|GetInputKeyTimeDown (Game|GetPlayerController 0) "SpaceBar") 0.0)
            (if (Variables|Default|GetOnWall?)
              (Variables|/Script/Engine.CharacterMovementComponent|SetGravityScale _charactermovement_2 0.0)
              (Class|MovementComponent|SetPlaneConstraintNormal _charactermovement_2 "0, 0,1.000000")
              (Physics|AddForce _charactermovement_2 (* (Variables|Default|GetPlayerDirection) 4000))
              (else
                (Variables|/Script/Engine.CharacterMovementComponent|SetGravityScale _charactermovement 1.0 :!label _label)
                (Class|MovementComponent|SetPlaneConstraintNormal _charactermovement "0, 0,0.000000")
                (Variables|Default|SetOnWall? false)))))))
    (:then_1
      (if (Actor|ActorHasTag "RunWall")
        (goto _label)))))

(event EventBeginPlay
  ;[1 1 1] Jump&doubleJump
  (Class|MovementComponent|SetPlaneConstraintEnabled (Variables|Character|GetCharacterMovement) false))

(event EventOnLanded
  (params (Hit :type Hit%20Result%20Structure%20%28by%20ref%29))
  ;[1 1 1] Jump&doubleJump
  (Utilities|FlowControl|DoN 2) ; enters at Reset
)

(event EventTick
  (params (DeltaSeconds :type Float%20%28single-precision%29))
  ;[1 1 1] Ledge_Climbing
  (bind _outhit (Collision|LineTraceByChannel (Transformation|GetActorLocation) (Transformation|GetWorldLocation (Variables|Default|GetEndLoc_WallClimb)) "TraceTypeQuery1" false 0 "None"))
  (if (Actor|ActorHasTag (.hitactor _outhit) "Climb_Wall_Able")
    (bind _output_get (Variables|Default|SetGiveClimbTime (Class|PlayerController|GetInputKeyTimeDown (Game|GetPlayerController 0) "SpaceBar")))
    (if (!= _output_get 0.0)
      (if (<= _output_get 0.7)
        (Character|LaunchCharacter "0, 0,500.000000" true true)))
    (else
      (Variables|Default|SetGiveClimbTime 0.0))))

(event Input|ActionEvents|InputActionJump
  (params (Key :type Key%20Structure :default "None"))
  ;[1 1 1] Jump&doubleJump
  (:Pressed
    (bind _counter (Utilities|FlowControl|DoN 2)
      (:Exit
        (switch int _counter
          (:1
            _)
          (:2
            _))
        (Character|LaunchCharacter "0, 0,450.000000" false true))))
  (:Released
    (Character|StopJumping)))

(event Input|ActionEvents|InputActionCrouch
  (params (Key :type Key%20Structure :default "None"))
  ;[1 1 1] Crouching
  (:Pressed
    (Character|StopJumping)))

(event Input|ActionEvents|InputActionClimbing
  (params (Key :type Key%20Structure :default "None"))
  ;[1 1 1] Ladder_Climbing
  (:Pressed
    (if (Variables|Default|GetNear%20Ladder?)
      (if (Variables|Default|GetLadder?)
        (Variables|Default|SetLadder? false)
        (Pawn|Components|CharacterMovement|SetMovementMode (Variables|Character|GetCharacterMovement) "MOVE_Walking" 0)
        (else
          (Variables|Default|SetLadder? true))))))

(event Input|AxisEvents|InputAxisForward_Backward
  (params (AxisValue :type Float%20%28single-precision%29))
  ;[1 1 1] Basic_Movement
  (if (== (Variables|Default|GetGiveClimbTime) 0.0)
    (if (Variables|Default|GetLadder?)
      (Pawn|Components|CharacterMovement|SetMovementMode (Variables|Character|GetCharacterMovement) "MOVE_Flying" 0)
      (Pawn|Input|AddMovementInput (Transformation|GetActorUpVector (Game|GetPlayerCharacter 0)) AxisValue false)
      (else
        (Pawn|Input|AddMovementInput (Math|Vector|GetForwardVector (Pawn|GetControlRotation :!class /Script/Engine.Pawn)) AxisValue false)))))

(event Input|AxisEvents|InputAxisLook_Left_Right
  (params (AxisValue :type Float%20%28single-precision%29))
  ;[1 1 1] Basic_Look
  (if (== (Variables|Default|GetGiveClimbTime) 0.0)
    (Pawn|Input|AddControllerYawInput AxisValue)))

(event Input|AxisEvents|InputAxisLook_Up_Down
  (params (AxisValue :type Float%20%28single-precision%29))
  ;[1 1 1] Basic_Look
  (if (== (Variables|Default|GetGiveClimbTime) 0.0)
    (Pawn|Input|AddControllerPitchInput AxisValue)))

(event Input|AxisEvents|InputAxisLeft_Right
  (params (AxisValue :type Float%20%28single-precision%29))
  ;[1 1 1] Basic_Movement
  (if (== (Variables|Default|GetGiveClimbTime) 0.0)
    (Pawn|Input|AddMovementInput (Math|Vector|GetRightVector (Pawn|GetControlRotation :!class /Script/Engine.Pawn)) AxisValue false)))

(fn ConstructionScript)